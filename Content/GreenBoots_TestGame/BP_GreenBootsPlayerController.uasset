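; Player controller for the GreenBoots test game that provides mouse click-to-move navigation for BP_GreenBootsCharacter.
; It stores the possessed pawn, then on BeginPlay sets Game and UI input, points the view at that pawn, and shows a custom WBP_MouseCursor widget as the cursor.
; Left click traces under the cursor on the Visibility channel and passes the hit location to the character's MoveToLocation.
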(event `self.ReceivePossess`
  (params (PossessedPawn :type "Pawn Object Reference"))
  ;[1 1 1] Mouse click navigation
  (set `self.Possessed Pawn` PossessedPawn))

(event `ClientInitialize`)

(event `self.ReceiveBeginPlay`
  ;[1 1 1] Mouse click navigation
  (`WidgetBlueprintLibrary.SetInputMode_GameAndUIEx` self null "DoNotLock" false)
  (`self.SetViewTargetWithBlend` (`self.Possessed Pawn`))
  (bind _returnvalue (`|CreateWidget` "/Game/GreenBoots_TestGame/Widgets/WBP_MouseCursor.WBP_MouseCursor_C"))
  (`self.SetMouseCursorWidget` "Default" _returnvalue)
  (set `self.bShowMouseCursor` true))

(event `Key|LeftMouseButton`
  (params (Key :type "Key Structure"))
  ;[1 1 1] Mouse click navigation
  (:`Pressed`
    (bind _asbp_green_boots_character (cast `/Game/GreenBoots_TestGame/Character/BP_GreenBootsCharacter` (`self.Possessed Pawn`)))
    (`/Game/GreenBoots_TestGame/Character/BP_GreenBootsCharacter.MoveToLocation` _asbp_green_boots_character (`.Location` (`GameplayStatics.BreakHitResult` (`self.GetHitResultUnderCursorByChannel` "TraceTypeQuery1"))))))

(fn `UserConstructionScript`)